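; BP_Terminal is an interactive terminal actor that shows a UI widget to a player character inside its Box volume.
; It creates the widget once on BeginPlay and keeps it for reuse.
; A Select event adds it to the viewport if the first found ThirdPersonCharacter or ThirdPersonCharacter_Controller overlaps the Box.
; End overlap by either character type removes the widget.
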(event OnComponentEndOverlap(Box)
  (params (OverlappedComponent :type Primitive%20Component%20Object%20Reference) (OtherActor :type Actor%20Object%20Reference) (OtherComp :type Primitive%20Component%20Object%20Reference) (OtherBodyIndex :type Integer))
  (Utilities|FlowControl|Sequence
    (:then_0
      (Utilities|Casting|CastToThirdPersonCharacter OtherActor))
    (:then_1
      (Utilities|Casting|CastToThirdPersonCharacter_Controller OtherActor)))
  (Widget|RemovefromParent (Variables|Default|GetWidget)))

(event Custom|CreateWidget
  (bind _returnvalue (UserInterface|CreateWidget "/Game/Terminal/Widget.Widget_C"))
  (Variables|Default|SetWidget _returnvalue))

(event Custom|Select
  (Utilities|FlowControl|Sequence
    (:then_0
      (bind _outactors (Actor|GetAllActorsOfClass "/Game/ThirdPersonBP/Blueprints/ThirdPersonCharacter.ThirdPersonCharacter_C")))
    (:then_1
      (bind _outactors_2 (Actor|GetAllActorsOfClass "/Game/ThirdPersonBP/Blueprints/ThirdPersonCharacter_Controller.ThirdPersonCharacter_Controller_C"))))
  (if (or (Collision|IsOverlappingActor (Variables|Default|GetBox) (Utilities|Array|Get(acopy) _outactors) :!class /Script/Engine.PrimitiveComponent) (Collision|IsOverlappingActor (Variables|Default|GetBox) (Utilities|Array|Get(acopy) _outactors_2) :!class /Script/Engine.PrimitiveComponent))
    (UserInterface|Viewport|AddtoViewport (Variables|Default|GetWidget) 0)))

(event EventBeginPlay
  (CallFunction|CreateWidget))

(fn ConstructionScript)