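; BP_Strahovka is a lobby display object with a platform, circle and money component, named after the Russian word for insurance.
; Tick spins the platform steadily around yaw.
; BeginPlay caches the money's relative location for the Anim timeline, whose update would roll the circle and move and roll the money.
; Nothing in this graph starts that timeline's exec inputs, so only the platform spin is driven here.
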(event EventTick
  (params (DeltaSeconds :type Float%20%28single-precision%29))
  (Transformation|AddLocalRotation (Variables|Default|GetS_Platform) (Math|Rotator|MakeRotator 0.0 0.0 (* DeltaSeconds 2e+01)) false false))

(event EventBeginPlay
  (Variables|Default|SetSircle%20Relative%20Location (Variables|/Script/Engine.SceneComponent|GetRelativeLocation (Variables|Default|GetS_Money))))

(fn ConstructionScript)