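; BP_Birja is a lobby prop with a rotating 3D object and seven graph meshes.
; Tick spins the main object around yaw at a constant, frame-rate-independent speed.
; A GraphMovement timeline is set up to stretch the graph meshes vertically in three groups, each driven by its own track, but nothing starts it, so only the rotation runs.
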(event EventTick
  (params (DeltaSeconds :type Float%20%28single-precision%29))
  (Transformation|AddLocalRotation (Variables|Default|GetS_Object3_S_Object3) (Math|Rotator|MakeRotator 0.0 0.0 (* DeltaSeconds 2e+01)) false false))

(fn ConstructionScript)