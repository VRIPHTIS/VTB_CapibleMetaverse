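; Lobby carousel of VTB bank products that shows a widget and web link for the featured one.
; BeginPlay gathers actors tagged "Products" and BP_ProductsPosition markers, then runs the first rotation.
; Each rotation shifts products one slot, enlarges the one sent to the last slot, and picks its widget and URL by class casts.
; Next rotates and OpenLink launches the URL, both gated on ThirdPersonCharacter overlapping the Box.
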(event Custom|OpenLink
  (for _array_element (Collision|GetOverlappingActors (Variables|Default|GetBox) 0 :!class /Script/Engine.PrimitiveComponent)
    (Utilities|Casting|CastToThirdPersonCharacter _array_element)
    (Utilities|Platform|LaunchURL (Variables|Default|GetLink))))

(event Custom|Next
  (bind _productspos (Variables|Default|GetProductsPos))
  (bind _products (Variables|Default|GetProducts))
  (bind _returnvalue (Utilities|Array|Length _products))
  (bind _returnvalue_2 (- _returnvalue 1))
  (for _array_element (Collision|GetOverlappingActors (Variables|Default|GetBox) 0 :!class /Script/Engine.PrimitiveComponent)
    (Utilities|Casting|CastToThirdPersonCharacter _array_element)
    (Variables|Default|SetCurrentProduct (Utilities|Array|Get(acopy) (Variables|Default|GetProducts)))
    (for _index (range 1 (- (Utilities|Array|Length (Variables|Default|GetProducts)) 1))
      (Transformation|SetActorTransform (Utilities|Array|Get(acopy) (Variables|Default|GetProducts) _index) (Math|Transform|MakeTransform (Transformation|GetActorLocation (Utilities|Array|Get(acopy) (Variables|Default|GetProductsPos) (+ _index -1))) "0, 0, 0" "0.600000,0.600000,0.600000")))
    (Transformation|SetActorTransform (Utilities|Array|Get(acopy) (Variables|Default|GetProducts)) (Math|Transform|MakeTransform (Transformation|GetActorLocation (Utilities|Array|Get(acopy) _productspos (- (Utilities|Array|Length _productspos) 1))) "0, 0, 0" "1.200000,1.200000,1.200000"))
    (for _index_2 (range 1 _returnvalue_2)
      (Utilities|Array|SetArrayElem _products (- _index_2 1) (Utilities|Array|Get(acopy) _products _index_2)))
    (Utilities|Array|SetArrayElem _products _returnvalue_2 (Variables|Default|GetCurrentProduct))
    (Variables|Default|SetNewVar_0 0)
    (Utilities|FlowControl|Sequence
      (:then_0
        (Utilities|Casting|CastToBP_VTB_ID (Variables|Default|GetCurrentProduct))
        (bind _returnvalue_3 (UserInterface|CreateWidget "/Game/Migrate/Lobby/ObjectLogic/VTB_ID/BTB_ID_Widget.BTB_ID_Widget_C"))
        (UserInterface|SetWidget (Variables|Default|GetWidget) _returnvalue_3)
        (Variables|Default|SetLink "https://www.vtb.ru/personal/online-servisy/vtb-id/"))
      (:then_1
        (Utilities|Casting|CastToBP_Birja (Variables|Default|GetCurrentProduct))
        (bind _returnvalue_4 (UserInterface|CreateWidget "/Game/Migrate/Lobby/ObjectLogic/BirjaMemov/BirjaWidget.BirjaWidget_C"))
        (UserInterface|SetWidget (Variables|Default|GetWidget) _returnvalue_4)
        (Variables|Default|SetLink "https://www.vtb.ru/personal/investicii/"))
      (:then_2
        (Utilities|Casting|CastToBP_Invest (Variables|Default|GetCurrentProduct))
        (bind _returnvalue_5 (UserInterface|CreateWidget "/Game/Migrate/Lobby/ObjectLogic/Invest/InvestWidget.InvestWidget_C"))
        (UserInterface|SetWidget (Variables|Default|GetWidget) _returnvalue_5)
        (Variables|Default|SetLink "https://www.vtb.ru/personal/vklady-i-scheta/"))
      (:then_3
        (Utilities|Casting|CastToBP_ObmenValut (Variables|Default|GetCurrentProduct))
        (bind _returnvalue_6 (UserInterface|CreateWidget "/Game/Migrate/Lobby/ObjectLogic/ObmenValut/ObmenWalutWidget.ObmenWalutWidget_C"))
        (UserInterface|SetWidget (Variables|Default|GetWidget) _returnvalue_6)
        (Variables|Default|SetLink "https://www.vtb.ru/personal/platezhi-i-perevody/obmen-valjuty/"))
      (:then_4
        (Utilities|Casting|CastToBP_Oformlenie (Variables|Default|GetCurrentProduct))
        (bind _returnvalue_7 (UserInterface|CreateWidget "/Game/Migrate/Lobby/ObjectLogic/OformlenieBuissiness/OformlenieBiusinessWidget.OformlenieBiusinessWidget_C"))
        (UserInterface|SetWidget (Variables|Default|GetWidget) _returnvalue_7)
        (Variables|Default|SetLink "https://www.vtb.ru/malyj-biznes/registraciya/"))
      (:then_5
        (Utilities|Casting|CastToBP_Strahovka (Variables|Default|GetCurrentProduct))
        (bind _returnvalue_8 (UserInterface|CreateWidget "/Game/Migrate/Lobby/ObjectLogic/Strahovka/StrakhovkaWidget.StrakhovkaWidget_C"))
        (UserInterface|SetWidget (Variables|Default|GetWidget) _returnvalue_8)
        (Variables|Default|SetLink "https://www.vtb.ru/personal/drugie-uslugi/strahovye-i-servisnye-produkty/"))
      (:then_6
        (Utilities|Casting|CastToBP_8 (Variables|Default|GetCurrentProduct))
        (bind _returnvalue_9 (UserInterface|CreateWidget "/Game/Migrate/Lobby/ObjectLogic/Vkladi/VkladiWidget.VkladiWidget_C"))
        (UserInterface|SetWidget (Variables|Default|GetWidget) _returnvalue_9)
        (Variables|Default|SetLink "https://www.vtb.ru/personal/vklady-i-scheta/"))
      (:then_7
        (Utilities|Casting|CastToBP_Ipoteka (Variables|Default|GetCurrentProduct))
        (UserInterface|CreateWidget "/Game/Migrate/Lobby/ObjectLogic/Ipoteka/IpotekaWidget.IpotekaWidget_C")
        (UserInterface|SetWidget (Variables|Default|GetWidget) 0)
        (Variables|Default|SetLink "https://www.vtb.ru/personal/ipoteka/"))
      (:then_8
        (Utilities|Casting|CastToBP_Businness (Variables|Default|GetCurrentProduct))
        (bind _returnvalue_10 (UserInterface|CreateWidget "/Game/Migrate/Lobby/ObjectLogic/Buiseness/Businnes.Businnes_C"))
        (UserInterface|SetWidget (Variables|Default|GetWidget) _returnvalue_10)
        (Variables|Default|SetLink "https://www.vtb.ru/malyj-biznes/")))))

(event EventBeginPlay
  (bind _outactors (Actor|GetAllActorsOfClass "/Game/Migrate/Lobby/ObjectLogic/BP_ProductsPosition.BP_ProductsPosition_C"))
  (Variables|Default|SetProductsPos _outactors)
  (bind _outactors_2 (Actor|GetAllActorswithTag "Products"))
  (bind _output_get (Variables|Default|SetProducts _outactors_2))
  (for (_array_element _array_index) (Variables|Default|GetProductsPos)
    (Transformation|SetActorTransform (Utilities|Array|Get(acopy) _output_get _array_index) (Math|Transform|MakeTransform (.location (Transformation|GetActorTransform _array_element)) "0, 0, 0" "0.600000,0.600000,0.600000")))
  (Variables|Default|SetCurrentProduct (Utilities|Array|Get(acopy) (Variables|Default|GetProducts)))
  (Variables|Default|SetCurrentProduct (Utilities|Array|Get(acopy) (Variables|Default|GetProducts)))
  (for _index (range 1 (- (Utilities|Array|Length (Variables|Default|GetProducts)) 1))
    (Transformation|SetActorTransform (Utilities|Array|Get(acopy) (Variables|Default|GetProducts) _index) (Math|Transform|MakeTransform (Transformation|GetActorLocation (Utilities|Array|Get(acopy) (Variables|Default|GetProductsPos) (+ _index -1))) "0, 0, 0" "0.600000,0.600000,0.600000")))
  (Transformation|SetActorTransform (Utilities|Array|Get(acopy) (Variables|Default|GetProducts)) (Math|Transform|MakeTransform (Transformation|GetActorLocation (Utilities|Array|Get(acopy) (Variables|Default|GetProductsPos) (- (Utilities|Array|Length (Variables|Default|GetProductsPos)) 1))) "0, 0, 0" "1.200000,1.200000,1.200000"))
  (for _index_2 (range 1 (- (Utilities|Array|Length (Variables|Default|GetProducts)) 1))
    (Utilities|Array|SetArrayElem (Variables|Default|GetProducts) (- _index_2 1) (Utilities|Array|Get(acopy) (Variables|Default|GetProducts) _index_2)))
  (Utilities|Array|SetArrayElem (Variables|Default|GetProducts) (- (Utilities|Array|Length (Variables|Default|GetProducts)) 1) (Variables|Default|GetCurrentProduct))
  (Variables|Default|SetNewVar_0 0)
  (Utilities|FlowControl|Sequence
    (:then_0
      (Utilities|Casting|CastToBP_VTB_ID (Variables|Default|GetCurrentProduct))
      (bind _returnvalue (UserInterface|CreateWidget "/Game/Migrate/Lobby/ObjectLogic/VTB_ID/BTB_ID_Widget.BTB_ID_Widget_C"))
      (UserInterface|SetWidget (Variables|Default|GetWidget) _returnvalue)
      (Variables|Default|SetLink "https://www.vtb.ru/personal/online-servisy/vtb-id/"))
    (:then_1
      (Utilities|Casting|CastToBP_Birja (Variables|Default|GetCurrentProduct))
      (bind _returnvalue_2 (UserInterface|CreateWidget "/Game/Migrate/Lobby/ObjectLogic/BirjaMemov/BirjaWidget.BirjaWidget_C"))
      (UserInterface|SetWidget (Variables|Default|GetWidget) _returnvalue_2)
      (Variables|Default|SetLink "https://www.vtb.ru/personal/investicii/"))
    (:then_2
      (Utilities|Casting|CastToBP_Invest (Variables|Default|GetCurrentProduct))
      (bind _returnvalue_3 (UserInterface|CreateWidget "/Game/Migrate/Lobby/ObjectLogic/Invest/InvestWidget.InvestWidget_C"))
      (UserInterface|SetWidget (Variables|Default|GetWidget) _returnvalue_3)
      (Variables|Default|SetLink "https://www.vtb.ru/personal/vklady-i-scheta/"))
    (:then_3
      (Utilities|Casting|CastToBP_ObmenValut (Variables|Default|GetCurrentProduct))
      (bind _returnvalue_4 (UserInterface|CreateWidget "/Game/Migrate/Lobby/ObjectLogic/ObmenValut/ObmenWalutWidget.ObmenWalutWidget_C"))
      (UserInterface|SetWidget (Variables|Default|GetWidget) _returnvalue_4)
      (Variables|Default|SetLink "https://www.vtb.ru/personal/platezhi-i-perevody/obmen-valjuty/"))
    (:then_4
      (Utilities|Casting|CastToBP_Oformlenie (Variables|Default|GetCurrentProduct))
      (bind _returnvalue_5 (UserInterface|CreateWidget "/Game/Migrate/Lobby/ObjectLogic/OformlenieBuissiness/OformlenieBiusinessWidget.OformlenieBiusinessWidget_C"))
      (UserInterface|SetWidget (Variables|Default|GetWidget) _returnvalue_5)
      (Variables|Default|SetLink "https://www.vtb.ru/malyj-biznes/registraciya/"))
    (:then_5
      (Utilities|Casting|CastToBP_Strahovka (Variables|Default|GetCurrentProduct))
      (bind _returnvalue_6 (UserInterface|CreateWidget "/Game/Migrate/Lobby/ObjectLogic/Strahovka/StrakhovkaWidget.StrakhovkaWidget_C"))
      (UserInterface|SetWidget (Variables|Default|GetWidget) _returnvalue_6)
      (Variables|Default|SetLink "https://www.vtb.ru/personal/drugie-uslugi/strahovye-i-servisnye-produkty/"))
    (:then_6
      (Utilities|Casting|CastToBP_8 (Variables|Default|GetCurrentProduct))
      (bind _returnvalue_7 (UserInterface|CreateWidget "/Game/Migrate/Lobby/ObjectLogic/Vkladi/VkladiWidget.VkladiWidget_C"))
      (UserInterface|SetWidget (Variables|Default|GetWidget) _returnvalue_7)
      (Variables|Default|SetLink "https://www.vtb.ru/personal/vklady-i-scheta/"))
    (:then_7
      (Utilities|Casting|CastToBP_Ipoteka (Variables|Default|GetCurrentProduct))
      (UserInterface|CreateWidget "/Game/Migrate/Lobby/ObjectLogic/Ipoteka/IpotekaWidget.IpotekaWidget_C")
      (UserInterface|SetWidget (Variables|Default|GetWidget) 0)
      (Variables|Default|SetLink "https://www.vtb.ru/personal/ipoteka/"))
    (:then_8
      (Utilities|Casting|CastToBP_Businness (Variables|Default|GetCurrentProduct))
      (bind _returnvalue_8 (UserInterface|CreateWidget "/Game/Migrate/Lobby/ObjectLogic/Buiseness/Businnes.Businnes_C"))
      (UserInterface|SetWidget (Variables|Default|GetWidget) _returnvalue_8)
      (Variables|Default|SetLink "https://www.vtb.ru/malyj-biznes/"))))

(event Collision|EventActorBeginOverlap
  (params (OtherActor :type Actor%20Object%20Reference)))

(event EventTick
  (params (DeltaSeconds :type Float%20%28single-precision%29)))

(fn ConstructionScript)