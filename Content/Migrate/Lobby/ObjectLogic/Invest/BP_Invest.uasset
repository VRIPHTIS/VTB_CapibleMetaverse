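; BP_Invest is a lobby prop made of cylinder meshes and a platform, apparently themed around investment.
; Tick continuously spins the platform around its yaw axis at a constant, frame-rate-independent speed.
; An unconnected timeline would stretch three groups of these components vertically on separate rise curves, but nothing triggers it.
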(event EventTick
  (params (DeltaSeconds :type Float%20%28single-precision%29))
  (Transformation|AddLocalRotation (Variables|Default|GetS_Object6_S_Platform_009) (Math|Rotator|MakeRotator 0.0 0.0 (* DeltaSeconds 2e+01)) false false))

(fn ConstructionScript)