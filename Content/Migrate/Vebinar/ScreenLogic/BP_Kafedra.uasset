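; BP_Kafedra is a lectern that lets the player page through presentation slides in a webinar scene.
; An overlap volume enables slide control while a ThirdPersonCharacter stands inside it.
; Forward and backward press events step a bounded slide number and broadcast it to every widget implementing BPI_SlideChange.
; StopSlidePlay and the lectern's own ChangeSlideNumber function are empty stubs.
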(event OnComponentBeginOverlap(Col_PresentSpace)
  (params (OverlappedComponent :type Primitive%20Component%20Object%20Reference) (OtherActor :type Actor%20Object%20Reference) (OtherComp :type Primitive%20Component%20Object%20Reference) (OtherBodyIndex :type Integer) (bFromSweep :type Boolean) (SweepResult :type Hit%20Result%20Structure%20%28by%20ref%29))
  (Utilities|Casting|CastToThirdPersonCharacter OtherActor)
  (Variables|Default|SetPresentationStarted? true))

(event OnComponentEndOverlap(Col_PresentSpace)
  (params (OverlappedComponent :type Primitive%20Component%20Object%20Reference) (OtherActor :type Actor%20Object%20Reference) (OtherComp :type Primitive%20Component%20Object%20Reference) (OtherBodyIndex :type Integer))
  (Utilities|Casting|CastToThirdPersonCharacter OtherActor)
  (Variables|Default|SetPresentationStarted? false))

(event Custom|Forward%20Slide%20Pressed
  (bind _choosenslidenumber (Variables|Default|GetChoosenSlideNumber))
  (if (and (< _choosenslidenumber 5) (Variables|Default|GetPresentationStarted?))
    (Math|Integer|IncrementInt _choosenslidenumber
      (:%20%20
        (bind _foundwidgets (Class|WidgetBlueprintLibrary|GetAllWidgetswithInterface "/Game/Migrate/Vebinar/ScreenLogic/BPI_SlideChange.BPI_SlideChange_C" false))
        (Class|BPISlideChange|ChangeSlideNumber(Message) _foundwidgets (Variables|Default|GetChoosenSlideNumber))))))

(event Custom|Backward%20Button%20Pressed
  (bind _choosenslidenumber (Variables|Default|GetChoosenSlideNumber))
  (if (and (> _choosenslidenumber 0) (Variables|Default|GetPresentationStarted?))
    (Math|Integer|DecrementInt _choosenslidenumber
      (:%20%20
        (bind _foundwidgets (Class|WidgetBlueprintLibrary|GetAllWidgetswithInterface "/Game/Migrate/Vebinar/ScreenLogic/BPI_SlideChange.BPI_SlideChange_C" false))
        (Class|BPISlideChange|ChangeSlideNumber(Message) _foundwidgets (Variables|Default|GetChoosenSlideNumber))))))

(event Custom|Stop%20Slide%20Play)

(fn ConstructionScript)

(fn ChangeSlideNumber
  (params (NewSlideNumber :type Integer))
  (return false))