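; Tree actor that scales up as it grows, accrues cash, and can be killed with a leaf burst.
; A timeline drives root scale from BeginPlay and passes the tree to ThirdPersonCharacter's TreeGrowth when finished.
; Tick polls that character's Minus flag to run or pause growth, adding Cash to TotalCash every three seconds while set.
; KillTree plays a second scale timeline, activates the colored LeafeExplosion effect, then destroys the actor.
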(event Custom|KillTree
  (bind _scaler (Timeline|TreeKill PlayFromStart)
    (:Update
      (Transformation|SetWorldScale3D (Variables|Default|GetDefaultSceneRoot) (Math|Conversions|ToVector(Float) _scaler))
      (Niagara|SetNiagaraVariable(LinearColor) (Variables|Default|GetLeafeExplosion) "ColorChange" (Variables|Default|GetLinearColorNS))
      (Components|Activation|Activate (Variables|Default|GetLeafeExplosion) false))
    (:Finished
      (Actor|DestroyActor))))

(event EventBeginPlay
  (bind _newtrack_0 (Timeline|TreeGrowth PlayFromStart)
    (:Update
      (Transformation|SetWorldScale3D (Variables|Default|GetDefaultSceneRoot) (Math|Vector|MakeVector _newtrack_0 _newtrack_0 _newtrack_0)))
    (:Finished
      (bind _outactors (Actor|GetAllActorsOfClass "/Game/ThirdPersonBP/Blueprints/ThirdPersonCharacter.ThirdPersonCharacter_C"))
      (Default|TreeGrowth (Utilities|Array|Get(acopy) _outactors) self))))

(event EventTick
  (params (DeltaSeconds :type Float%20%28single-precision%29))
  (bind _outactors (Actor|GetAllActorsOfClass "/Game/ThirdPersonBP/Blueprints/ThirdPersonCharacter.ThirdPersonCharacter_C"))
  (if (Variables|/Game/ThirdPersonBP/Blueprints/ThirdPersonCharacter.ThirdPersonCharacter_C|GetMinus (Utilities|Array|Get(acopy) _outactors))
    (Components|Timeline|SetPlayRate (Variables|Default|GetTreeGrowth) 1.0)
    (bind _output_get (Variables|Default|SetDeltaTimeCash (+ DeltaSeconds (Variables|Default|GetDeltaTimeCash))))
    (if (>= _output_get 3.0)
      (Variables|Default|SetDeltaTimeCash 0.0)
      (Variables|Default|SetTotalCash (+ (Variables|Default|GetCash) (Variables|Default|GetTotalCash))))
    (else
      (Components|Timeline|SetPlayRate (Variables|Default|GetTreeGrowth) 0.0))))

(fn ConstructionScript)