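; BP_TeleportLobbyGames is a trigger actor that starts a player teleport, named for the lobby games.
; On Box overlap, it skips if TeleportHandler already has a teleport in process, then checks that the overlapping actor's first tag is "Player".
; It sets that actor as the handler's TargetActor and calls TeleportPerson, leaving the destination and move logic to TeleportHandler.
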(event OnComponentBeginOverlap(Box)
  (params (OverlappedComponent :type Primitive%20Component%20Object%20Reference) (OtherActor :type Actor%20Object%20Reference) (OtherComp :type Primitive%20Component%20Object%20Reference) (OtherBodyIndex :type Integer) (bFromSweep :type Boolean) (SweepResult :type Hit%20Result%20Structure%20%28by%20ref%29))
  (bind _teleporthandler (Variables|Default|GetTeleportHandler))
  (if (not (Variables|/Game/Teleport/BP_TeleportHandler.BP_TeleportHandler_C|GetTeleportationInProcess (Variables|Default|GetTeleportHandler)))
    (if (Utilities|Name|Equal(Name) (Utilities|Array|Get(acopy) (Variables|/Script/Engine.Actor|GetTags OtherActor)) "Player")
      (Variables|/Game/Teleport/BP_TeleportHandler.BP_TeleportHandler_C|SetTargetActor _teleporthandler OtherActor)
      (Default|TeleportPerson _teleporthandler))))

(event EventBeginPlay
  (|CallParentFunction) ; This node is disabled and will not be called.\nDrag off pins to build functionality.
)

(event Collision|EventActorBeginOverlap
  (params (OtherActor :type Actor%20Object%20Reference))
  (|CallParentFunction OtherActor) ; This node is disabled and will not be called.\nDrag off pins to build functionality.
)

(event EventTick
  (params (DeltaSeconds :type Float%20%28single-precision%29))
  (|CallParentFunction DeltaSeconds) ; This node is disabled and will not be called.\nDrag off pins to build functionality.
)

(fn ConstructionScript
  (|CallParentFunction))