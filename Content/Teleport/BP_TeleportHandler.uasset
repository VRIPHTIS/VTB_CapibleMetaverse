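; BP_TeleportHandler is a Blueprint that moves a target actor to an end teleport.
; Its TeleportPerson event checks the end teleport and target references, then places the actor at the end teleport's Box location without sweep.
; A TeleportationInProcess flag blocks repeat calls and is never cleared here.
; The debug print and the clearing of references are disconnected and never run.
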(event Custom|TeleportPerson
  (if (not (Variables|Default|GetTeleportationInProcess))
    (Variables|Default|SetTeleportationInProcess true)
    (if (Math|Boolean|ANDBoolean true (Utilities|IsValid (Variables|Default|GetEndTeleport)) (Utilities|IsValid (Variables|Default|GetTargetActor)))
      (bind _output_get (Variables|Default|SetTargetLocation (Transformation|GetWorldLocation (Variables|/Game/Teleport/BP_Teleport.BP_Teleport_C|GetBox (Variables|Default|GetEndTeleport)))))
      (Transformation|SetActorLocation (Variables|Default|GetTargetActor) _output_get false true))))

(fn ConstructionScript)