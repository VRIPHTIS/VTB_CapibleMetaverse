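; BP_Teleport is a teleport point actor that signals when a teleportation ends.
; On BeginPlay it caches the first BP_TeleportHandler in the level, which holds the shared teleport state.
; When anything leaves its Box and this actor is the handler's EndTeleport, it clears the handler's TeleportationInProcess flag and TargetActor.
; Starting or performing the teleport is not handled here.
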(event OnComponentEndOverlap(Box)
  (params (OverlappedComponent :type Primitive%20Component%20Object%20Reference) (OtherActor :type Actor%20Object%20Reference) (OtherComp :type Primitive%20Component%20Object%20Reference) (OtherBodyIndex :type Integer))
  (bind _teleporthandler (Variables|Default|GetTeleportHandler))
  (if (== self (Variables|/Game/Teleport/BP_TeleportHandler.BP_TeleportHandler_C|GetEndTeleport _teleporthandler))
    (Variables|/Game/Teleport/BP_TeleportHandler.BP_TeleportHandler_C|SetTeleportationInProcess _teleporthandler false)
    (Variables|/Game/Teleport/BP_TeleportHandler.BP_TeleportHandler_C|SetTargetActor _teleporthandler 0)))

(event EventBeginPlay
  (bind _outactors (Actor|GetAllActorsOfClass "/Game/Teleport/BP_TeleportHandler.BP_TeleportHandler_C"))
  (Variables|Default|SetTeleportHandler (Utilities|Array|Get(acopy) _outactors)))

(event Collision|EventActorBeginOverlap
  (params (OtherActor :type Actor%20Object%20Reference)))

(event EventTick
  (params (DeltaSeconds :type Float%20%28single-precision%29)))

(fn ConstructionScript)