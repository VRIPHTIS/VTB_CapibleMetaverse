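; BP_Doors is a double sliding door that opens when the player enters its trigger and closes when they leave.
; Col_Door overlap events filter on the actor's first tag being "Player", then play or reverse the DoorOpenAnim timeline.
; The timeline's single track drives the relative Y position of both door panels, negated for the right one so they move in opposite directions.
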(event OnComponentBeginOverlap(Col_Door)
  (params (OverlappedComponent :type Primitive%20Component%20Object%20Reference) (OtherActor :type Actor%20Object%20Reference) (OtherComp :type Primitive%20Component%20Object%20Reference) (OtherBodyIndex :type Integer) (bFromSweep :type Boolean) (SweepResult :type Hit%20Result%20Structure%20%28by%20ref%29))
  (if (Utilities|Name|Equal(Name) (Utilities|Array|Get(acopy) (Variables|/Script/Engine.Actor|GetTags OtherActor)) "Player")
    (bind _newtrack_0 (Timeline|DoorOpenAnim Play)
      (:Update
        (Transformation|SetRelativeLocation (Variables|Default|GetS_DoorLeft) (Math|Vector|MakeVector 0.0 _newtrack_0 0.0) false false)
        (Transformation|SetRelativeLocation (Variables|Default|GetS_DoorRight) (Math|Vector|MakeVector 0.0 (* -1 _newtrack_0) 0.0) false false)))))

(event OnComponentEndOverlap(Col_Door)
  (params (OverlappedComponent :type Primitive%20Component%20Object%20Reference) (OtherActor :type Actor%20Object%20Reference) (OtherComp :type Primitive%20Component%20Object%20Reference) (OtherBodyIndex :type Integer))
  (if (Utilities|Name|Equal(Name) (Utilities|Array|Get(acopy) (Variables|/Script/Engine.Actor|GetTags OtherActor)) "Player")
    (bind _newtrack_0 (Timeline|DoorOpenAnim Reverse)
      (:Update
        (Transformation|SetRelativeLocation (Variables|Default|GetS_DoorLeft) (Math|Vector|MakeVector 0.0 _newtrack_0 0.0) false false)
        (Transformation|SetRelativeLocation (Variables|Default|GetS_DoorRight) (Math|Vector|MakeVector 0.0 (* -1 _newtrack_0) 0.0) false false)))))

(fn ConstructionScript)