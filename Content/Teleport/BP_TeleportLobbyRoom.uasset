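; BP_TeleportLobbyRoom is a lobby teleport trigger that routes overlapping actors to a room matching their input type.
; When its Box is entered and no teleport is in process, it checks the actor's second tag.
; "Mouse" targets the first BP_TeleportRoomThird and "Controller" the first BP_TeleportRoomVR found in the level.
; It passes that destination and the actor to TeleportHandler, which performs the teleport.
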(event OnComponentBeginOverlap(Box)
  (params (OverlappedComponent :type Primitive%20Component%20Object%20Reference) (OtherActor :type Actor%20Object%20Reference) (OtherComp :type Primitive%20Component%20Object%20Reference) (OtherBodyIndex :type Integer) (bFromSweep :type Boolean) (SweepResult :type Hit%20Result%20Structure%20%28by%20ref%29))
  (bind _tags (Variables|/Script/Engine.Actor|GetTags OtherActor))
  (bind _teleporthandler (Variables|Default|GetTeleportHandler))
  (bind _output (Utilities|Array|Get(acopy) _tags 1))
  (if (not (Variables|/Game/Teleport/BP_TeleportHandler.BP_TeleportHandler_C|GetTeleportationInProcess (Variables|Default|GetTeleportHandler)))
    (Utilities|FlowControl|Sequence
      (:then_0
        (if (Utilities|Name|Equal(Name) _output "Mouse")
          (bind _outactors (Actor|GetAllActorsOfClass "/Game/Teleport/Rooms/BP_TeleportRoomThird.BP_TeleportRoomThird_C"))
          (Variables|/Game/Teleport/BP_TeleportHandler.BP_TeleportHandler_C|SetEndTeleport _teleporthandler (Utilities|Array|Get(acopy) _outactors))
          (Variables|/Game/Teleport/BP_TeleportHandler.BP_TeleportHandler_C|SetTargetActor _teleporthandler OtherActor :!label _label)
          (Default|TeleportPerson _teleporthandler)))
      (:then_1
        (if (Utilities|Name|Equal(Name) _output "Controller")
          (bind _outactors_2 (Actor|GetAllActorsOfClass "/Game/Teleport/Rooms/BP_TeleportRoomVR.BP_TeleportRoomVR_C"))
          (Variables|/Game/Teleport/BP_TeleportHandler.BP_TeleportHandler_C|SetEndTeleport _teleporthandler (Utilities|Array|Get(acopy) _outactors_2))
          (goto _label))))))

(event EventBeginPlay
  (|CallParentFunction) ; This node is disabled and will not be called.\nDrag off pins to build functionality.
)

(event Collision|EventActorBeginOverlap
  (params (OtherActor :type Actor%20Object%20Reference))
  (|CallParentFunction OtherActor) ; This node is disabled and will not be called.\nDrag off pins to build functionality.
)

(event EventTick
  (params (DeltaSeconds :type Float%20%28single-precision%29))
  (|CallParentFunction DeltaSeconds) ; This node is disabled and will not be called.\nDrag off pins to build functionality.
)

(fn ConstructionScript
  (|CallParentFunction))