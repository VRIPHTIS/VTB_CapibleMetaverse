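; BP_Game2 runs a planting gamble minigame that scores the mushrooms, flowers and trees placed in BP_Pot actors.
; Player overlap with Review tallies pots by Cylinder mesh, adding to the counters without resetting them.
; Player overlap with Accept rolls a random loss or gain multiplier per type, with mushrooms riskiest and trees safest.
; It then sends counts, per-type net changes and the overall net to WBP_Game2's ShowResults.
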(event OnComponentBeginOverlap(Review)
  (params (OverlappedComponent :type Primitive%20Component%20Object%20Reference) (OtherActor :type Actor%20Object%20Reference) (OtherComp :type Primitive%20Component%20Object%20Reference) (OtherBodyIndex :type Integer) (bFromSweep :type Boolean) (SweepResult :type Hit%20Result%20Structure%20%28by%20ref%29))
  (Utilities|Casting|CastToThirdPersonCharacter OtherActor)
  (bind _outactors (Actor|GetAllActorsOfClass "/Game/InventorySystem/Pot/BP_Pot.BP_Pot_C"))
  (for _array_element _outactors
    (if (== (Variables|/Script/Engine.StaticMeshComponent|GetStaticMesh (Variables|/Game/InventorySystem/Pot/BP_Pot.BP_Pot_C|GetCylinder _array_element)) "/Game/InventorySystem/Pot/GardenAssets/Shrooms/s_blue_mashrom.s_blue_mashrom")
      (Math|Integer|IncrementInt (Variables|Default|GetAmmountOfShrooms))
      (elif (== (Variables|/Script/Engine.StaticMeshComponent|GetStaticMesh (Variables|/Game/InventorySystem/Pot/BP_Pot.BP_Pot_C|GetCylinder _array_element)) "/Game/InventorySystem/Pot/GardenAssets/Flower/s_blue_flower.s_blue_flower")
        (Math|Integer|IncrementInt (Variables|Default|GetAmmountOfFlowers))
        (elif (== (Variables|/Script/Engine.StaticMeshComponent|GetStaticMesh (Variables|/Game/InventorySystem/Pot/BP_Pot.BP_Pot_C|GetCylinder _array_element)) "/Game/InventorySystem/Pot/GardenAssets/Tree/s_b_tree.s_b_tree")
          (Math|Integer|IncrementInt (Variables|Default|GetAmmountOfTrees)))))))

(event OnComponentBeginOverlap(Accept)
  (params (OverlappedComponent :type Primitive%20Component%20Object%20Reference) (OtherActor :type Actor%20Object%20Reference) (OtherComp :type Primitive%20Component%20Object%20Reference) (OtherBodyIndex :type Integer) (bFromSweep :type Boolean) (SweepResult :type Hit%20Result%20Structure%20%28by%20ref%29))
  (Utilities|Casting|CastToThirdPersonCharacter OtherActor)
  (if (>= (Math|Random|RandomFloatinRange 0.0 1.0) 0.4)
    (Variables|Default|SetShroomResult (* (* (Variables|Default|GetAmmountOfShrooms) (Variables|Default|GetShroomsValue)) 0.4))
    (else
      (Variables|Default|SetShroomResult (* (* (Variables|Default|GetAmmountOfShrooms) (Variables|Default|GetShroomsValue)) 2.0))))
  (if (>= (Math|Random|RandomFloatinRange 0.0 1.0) 0.75)
    (Variables|Default|SetFlowerResult (* (* (Variables|Default|GetAmmountOfFlowers) (Variables|Default|GetFlowersValue)) 0.75))
    (else
      (Variables|Default|SetFlowerResult (* (* (Variables|Default|GetAmmountOfFlowers) (Variables|Default|GetFlowersValue)) 1.4))))
  (if (>= (Math|Random|RandomFloatinRange 0.0 1.0) 0.9)
    (Variables|Default|SetTreeResult (* (* (Variables|Default|GetAmmountOfTrees) (Variables|Default|GetTreeValue)) 0.9))
    (else
      (Variables|Default|SetTreeResult (* (* (Variables|Default|GetAmmountOfTrees) (Variables|Default|GetTreeValue)) 1.1))))
  (bind _foundwidgets (Widget|GetAllWidgetsOfClass "/Game/InventorySystem/Pot/GardenAssets/Game2Widget/WBP_Game2.WBP_Game2_C" false))
  (Default|ShowResults _foundwidgets (Variables|Default|GetAmmountOfTrees) (Variables|Default|GetAmmountOfFlowers) (Variables|Default|GetAmmountOfShrooms) (- (Variables|Default|GetTreeResult) (Math|Conversions|ToFloat(Integer) (* (Variables|Default|GetAmmountOfTrees) (Variables|Default|GetTreeValue)))) (- (Variables|Default|GetFlowerResult) (Math|Conversions|ToFloat(Integer) (* (Variables|Default|GetAmmountOfFlowers) (Variables|Default|GetFlowersValue)))) (- (Variables|Default|GetShroomResult) (Math|Conversions|ToFloat(Integer) (* (Variables|Default|GetAmmountOfShrooms) (Variables|Default|GetShroomsValue)))) (- (+ (Variables|Default|GetShroomResult) (Variables|Default|GetFlowerResult) (Variables|Default|GetTreeResult)) (Math|Conversions|ToFloat(Integer) (+ (* (Variables|Default|GetAmmountOfTrees) (Variables|Default|GetTreeValue)) (* (Variables|Default|GetAmmountOfFlowers) (Variables|Default|GetFlowersValue)) (* (Variables|Default|GetAmmountOfShrooms) (Variables|Default|GetShroomsValue)))))))

(fn ConstructionScript)