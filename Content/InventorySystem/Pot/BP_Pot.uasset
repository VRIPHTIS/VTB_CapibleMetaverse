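; BP_Pot is a plant pot actor in the inventory system that shows a plant growing when an object is planted in it.
; PlantInPot stores the given object name and calls the Posadka event, which swaps the Cylinder mesh to a tree, mushroom or flower by matching that name.
; A shared Scale timeline then plays from the start, driving the mesh's relative scale to animate the growth.
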(event Custom|Posadka
  (if (Utilities|Enum|Equal(Enum) (Variables|Default|GetObject%20Name) "Tree")
    (Components|StaticMesh|SetStaticMesh (Variables|Default|GetCylinder) "/Game/InventorySystem/Pot/GardenAssets/Tree/s_b_tree.s_b_tree")
    (bind _newtrack_0 (Timeline|Scale PlayFromStart)
      (:Update
        (Transformation|SetRelativeScale3D (Variables|Default|GetCylinder) (Math|Conversions|ToVector(Float) _newtrack_0)))
      (:Finished))
    (elif (Utilities|Enum|Equal(Enum) (Variables|Default|GetObject%20Name) "Shroom")
      (Components|StaticMesh|SetStaticMesh (Variables|Default|GetCylinder) "/Game/InventorySystem/Pot/GardenAssets/Shrooms/s_blue_mashrom.s_blue_mashrom")
      (Timeline|Scale PlayFromStart)
      (elif (Utilities|Enum|Equal(Enum) (Variables|Default|GetObject%20Name) "Flower")
        (Components|StaticMesh|SetStaticMesh (Variables|Default|GetCylinder) "/Game/InventorySystem/Pot/GardenAssets/Flower/s_blue_flower.s_blue_flower")
        (Timeline|Scale PlayFromStart)))))

(fn ConstructionScript)

(fn PlantinPot
  (params (ObjectToPlant :type String))
  (Variables|Default|SetObject%20Name ObjectToPlant)
  (CallFunction|Posadka)
  (return 0))